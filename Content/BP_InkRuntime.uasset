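; Ink runtime Blueprint that runs a branching story and bridges it to an on-screen example widget.
; On BeginPlay it creates WBP_InkExample, binds its choice and restart delegates, then starts a BP_InkThread at the configured path.
; Display events forward lines, choices and the restart button to the widget.
; Choosing clears the widget and passes the index, shifted down by one, to the thread; restarting is delegated to the GameMode.
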(event `self.ReceiveBeginPlay`
  (`|ExecutionSequence`
    (:`then_0`
      ;[0 0 0] Setup UI 🖥
      (bind _returnvalue (`|CreateWidget` "/Game/UI/WBP_InkExample.WBP_InkExample_C" (`GameplayStatics.GetPlayerController` 0)))
      (bind _output_get (set `self.Widget` _returnvalue))
      (`UserWidget.AddToViewport` _output_get 0)
      (add `/Game/UI/WBP_InkExample.OnChoiceChoosen` (`self.Widget`) (`|CreateDelegate` :!event `ChooseChoice`))
      (add `/Game/UI/WBP_InkExample.OnRestartBtnClicked` (`self.Widget`) (`|CreateDelegate` :!event `RestartStory`)))
    (:`then_1`
      ;[0 0 0] Start Ink Runtime
      (`self.StartStory`))))

(event `/Game/BPI_InkRuntime.DisplayLine`
  (params (InkLine :type String))
  (`/Game/UI/WBP_InkExample.DisplayLine` (`self.Widget`) InkLine))

(event `/Game/BPI_InkRuntime.DisplayChoices`
  (params (ChoicesByIdx :type "Map of Integer to String"))
  (`/Game/UI/WBP_InkExample.DisplayChoices` (`self.Widget`) ChoicesByIdx))

(event `/Game/BPI_InkRuntime.DisplayRestartButton`
  (`/Game/UI/WBP_InkExample.DisplayRestartButton` (`self.Widget`)))

(fn `ChooseChoice`
  (params (ChoiceIdx :type Integer))
  (`/Game/UI/WBP_InkExample.RemoveAll` (`self.Widget`))
  (`InkThread.PickChoice` (`self.InkThread`) (- ChoiceIdx 1)))

(fn `RestartStory`
  (message `/Game/Core/BPI_GM_inkcppUE.Restart` (`GameplayStatics.GetGameMode`)))

(fn `StartStory`
  (bind _returnvalue (`self.Start` (`self.InkThreadClass`) (`self.StartPath`)))
  (bind _asbp_ink_thread (cast `/Game/BP_InkThread` _returnvalue))
  (set `self.InkThread` _asbp_ink_thread))

(fn `UserConstructionScript`)
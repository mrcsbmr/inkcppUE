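; BP_InkThread is an Ink story thread that forwards narrative events to its runtime for display.
; Each written line is passed straight through as a line message.
; Offered choices are rebuilt into an index-to-text map before being sent as a choices message.
; On shutdown, the thread asks the runtime to display a restart button.
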(event `self.OnLineWritten`
  (params (line :type String) (tags :type "TagList Object Reference"))
  (message `/Game/BPI_InkRuntime.DisplayLine` (`self.GetRuntime`) line))

(event `self.OnChoice`
  (params (choices :type "Array of Choice Object Reference (by ref)"))
  (`BlueprintMapLibrary.Map_Clear` (`self.Choices by Index`))
  (for _array_element choices
    (`BlueprintMapLibrary.Map_Add` (`self.Choices by Index`) (`Choice.GetIndex` _array_element) (`Choice.GetText` _array_element)))
  (message `/Game/BPI_InkRuntime.DisplayChoices` (`self.GetRuntime`) (`self.Choices by Index`)))

(event `self.OnShutdown`
  (message `/Game/BPI_InkRuntime.DisplayRestartButton` (`self.GetRuntime`)))